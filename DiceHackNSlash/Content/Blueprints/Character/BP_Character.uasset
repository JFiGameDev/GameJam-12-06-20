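; Player character Blueprint with camera-relative movement, weapon attacks and stamina-gated dodge rolls.
; Mouse input spins the mesh while idle, movement restores its startup transform, and attack press/release forwards to the BP_BaseWeapon child actor.
; Roll plays a forward montage when moving or a step-back otherwise, spending stamina through duplicate RollCheck macros.
; Tick flags low stamina and replenishes it outside rolls; BeginPlay creates Health and Stamina widgets.
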(event Custom|Mouse%20Rotate
  (params (Mouse%20X :type Float%20%28single-precision%29) (Mouse%20Y :type Float%20%28single-precision%29))
  (if (not (Utilities|HasMovementInput))
    (Transformation|AddRelativeRotation (Variables|Character|GetMesh) (Math|Rotator|MakeRotator 0.0 0.0 (+ Mouse%20X Mouse%20Y)) false false)))

(event Custom|Move%20Up/Down
  (params (X%20Input :type Float%20%28single-precision%29))
  (if (!= X%20Input 0.0)
    (Pawn|Input|AddMovementInput (Math|Vector|GetForwardVector (Variables|Default|GetCamera)) X%20Input false)
    (Transformation|SetRelativeTransform (Variables|Character|GetMesh) (Variables|Default|GetMeshTransformAtStartup) false false)))

(event Custom|Roll
  (if (not (Variables|Default|GetStaminaEmpty?))
    (if (not (AI|Components|NavMovement|IsFalling (Variables|Character|GetCharacterMovement)))
      (if (not (Animation|Montage|MontageIsPlaying (Components|SkeletalMesh|GetAnimInstance (Variables|Character|GetMesh)) "/Game/Blueprints/Animation/Step_Back_Roll_Montage.Step_Back_Roll_Montage"))
        (if (Utilities|HasMovementInput)
          (CallFunction|PlayHighPriorityMontage "/Game/Blueprints/Animation/Dodge_Small_Forward_Roll_Montage.Dodge_Small_Forward_Roll_Montage" "None" 1.0)
          (|RollCheck)
          (else
            (CallFunction|TryPlayAnimMontage "/Game/Blueprints/Animation/Step_Back_Roll_Montage.Step_Back_Roll_Montage" "None" 1.0)
            (|RollCheck_2)))))))

(event Custom|Attack
  (bind _asbp_base_weapon (Utilities|Casting|CastToBP_BaseWeapon (Variables|/Script/Engine.ChildActorComponent|GetChildActor (Variables|Default|GetWeapon))))
  (Default|Attack _asbp_base_weapon))

(event Custom|Attack%20Released
  (bind _asbp_base_weapon (Utilities|Casting|CastToBP_BaseWeapon (Variables|/Script/Engine.ChildActorComponent|GetChildActor (Variables|Default|GetWeapon))))
  (Default|AttackReleased _asbp_base_weapon))

(event Custom|Move%20Left/Right
  (params (Y%20Input :type Float%20%28single-precision%29))
  (if (!= Y%20Input 0.0)
    (Pawn|Input|AddMovementInput (Math|Vector|GetRightVector (Variables|Default|GetCamera)) Y%20Input false)
    (Transformation|SetRelativeTransform (Variables|Character|GetMesh) (Variables|Default|GetMeshTransformAtStartup) false false)))

(event Custom|Initialization
  (Variables|Default|SetMeshTransformAtStartup (Transformation|GetRelativeTransform (Variables|Character|GetMesh)))
  (bind _returnvalue (Game|ConstructObjectfromClass "/Game/UI/Health.Health_C" self))
  (bind _returnvalue_2 (Game|ConstructObjectfromClass "/Game/UI/Stamina.Stamina_C" self))
  (UserInterface|Viewport|AddtoViewport _returnvalue_2 0))

(event EventTick
  (params (DeltaSeconds :type Float%20%28single-precision%29))
  (if (<= (Variables|Default|GetStamina) 25.0)
    (Variables|Default|SetStaminaEmpty? true)
    (Utilities|FlowControl|Delay 0.25)
    (Variables|Default|SetStaminaEmpty? false))
  (if (not (Variables|Default|GetRolling?))
    (Utilities|FlowControl|Delay 0.05)
    (CallFunction|Replenish)))

(event EventBeginPlay
  (CallFunction|Initialization))

(fn ConstructionScript)

(fn PlayHighPriorityMontage
  (params (Montage :type Anim%20Montage%20Object%20Reference) (StartSectionName :type Name) (InPlayRate :type Float%20%28single-precision%29))
  (if (not (Animation|Montage|MontageIsPlaying (Components|SkeletalMesh|GetAnimInstance (Variables|Character|GetMesh)) Montage))
    (bind _output_get (Variables|Default|SetHighPriorityMontage Montage))
    (bind _returnvalue (Animation|PlayAnimMontage _output_get InPlayRate StartSectionName))
    (return _returnvalue)))

(fn TryPlayAnimMontage
  (params (Montage :type Anim%20Montage%20Object%20Reference) (StartSectionName :type Name) (InPlayRate :type Float%20%28single-precision%29))
  (if (not (Animation|Montage|MontageIsPlaying (Components|SkeletalMesh|GetAnimInstance (Variables|Character|GetMesh)) 0))
    (bind _returnvalue (Animation|PlayAnimMontage Montage InPlayRate StartSectionName))
    (return _returnvalue)))

(fn Replenish
  (if (>= (Variables|Default|GetStamina) 1e+02)
    (Variables|Default|SetStamina 1e+02)
    (else
      (Variables|Default|SetStamina (+ (Variables|Default|GetStamina) 1.0)))))

(fn GetDesiredRotation
  (if (Utilities|HasMovementInput)
    (return (Math|Conversions|RotationFromXVector (Class|Pawn|GetLastMovementInputVector)))
    (else
      (return (Transformation|GetActorRotation)))))

(fn StartRotatingwithLimit
  (params (MaxPossibleRotation :type Float%20%28single-precision%29) (MaxDegreesPerSecond :type Float%20%28single-precision%29))
  (return))