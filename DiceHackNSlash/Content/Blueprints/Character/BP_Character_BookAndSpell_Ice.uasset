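; Player character Blueprint for a book-and-spell ice caster that fires an ice spell on the Attack input.
; Pressing Attack plays the magic animation montage on the mesh.
; The montage's notify-begin adds an audio component and spawns an Ice_Spell actor in front of the character, placed and oriented by control rotation so it follows the aim.
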(event EventBeginPlay
  (|CallParentFunction) ; This node is disabled and will not be called.\nDrag off pins to build functionality.
)

(event Collision|EventActorBeginOverlap
  (params (OtherActor :type Actor%20Object%20Reference)))

(event EventTick
  (params (DeltaSeconds :type Float%20%28single-precision%29))
  (|CallParentFunction DeltaSeconds) ; This node is disabled and will not be called.\nDrag off pins to build functionality.
)

(event Input|ActionEvents|InputActionAttack
  (params (Key :type Key%20Structure :default "None"))
  (bind _returnvalue (Pawn|GetControlRotation :!class /Script/Engine.Pawn))
  (:Pressed
    (Animation|Montage|PlayMontage (Variables|Character|GetMesh) "/Game/Character/Animations/Magic_Anim_Montage.Magic_Anim_Montage"
      (:OnNotifyBegin
        (AddComponent|AddAudioComponent false)
        (Game|SpawnActorfromClass "/Game/Blueprints/Ice_Spell.Ice_Spell_C" (Math|Transform|MakeTransform (+ (Transformation|GetActorLocation) (* (Math|Vector|GetForwardVector _returnvalue) 1.5e+02)) _returnvalue) "Undefined" 0 0)))))

(fn ConstructionScript
  (|CallParentFunction))