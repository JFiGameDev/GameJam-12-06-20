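; Spear-and-shield character Blueprint with a left-click spear attack and a right-click shield block, both driven by montage notifies.
; The attack notify runs a debug-drawn sphere trace from the collision component, then applies damage to the hit actor and reports a damage event.
; The block notify sets CanTakeDamage to true for the block duration, then back to false.
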(event EventBeginPlay
  (|CallParentFunction) ; This node is disabled and will not be called.\nDrag off pins to build functionality.
)

(event Collision|EventActorBeginOverlap
  (params (OtherActor :type Actor%20Object%20Reference)))

(event EventTick
  (params (DeltaSeconds :type Float%20%28single-precision%29))
  (|CallParentFunction DeltaSeconds) ; This node is disabled and will not be called.\nDrag off pins to build functionality.
)

(event Input|MouseEvents|RightMouseButton
  (params (Key :type Key%20Structure :default "None"))
  (:Pressed
    (Animation|Montage|PlayMontage (Variables|Character|GetMesh) "/Game/Character/Animations/Shield_Block_Anim_Montage.Shield_Block_Anim_Montage"
      (:OnNotifyBegin
        (Variables|Default|SetcanTakeDamage? true)
        (Utilities|FlowControl|Delay (Variables|Default|GetShieldBlockDuration))
        (Variables|Default|SetcanTakeDamage? false)))))

(event Input|MouseEvents|LeftMouseButton
  (params (Key :type Key%20Structure :default "None"))
  (bind _collisioncomponent (Variables|Default|GetCollisionComponent))
  (bind _returnvalue (Transformation|GetWorldLocation _collisioncomponent))
  (:Pressed
    (Animation|Montage|PlayMontage (Variables|Character|GetMesh) "/Game/Character/Animations/Spear_Anim_Montage.Spear_Anim_Montage"
      (:OnNotifyBegin
        (bind _outhit (Collision|SphereTraceByChannel _returnvalue (* (+ _returnvalue (Math|Vector|GetForwardVector (Transformation|GetActorRotation))) 1e+02) 4e+01 "TraceTypeQuery2" false 0 "Persistent"))
        (Game|Damage|ApplyDamage (.hitactor _outhit) 0.5 0 0)
        (Class|AISenseDamage|ReportDamageEvent (.hitactor _outhit) self 0.0 (.tracestart _outhit))))))

(fn ConstructionScript
  (|CallParentFunction))