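; Character Blueprint with helper functions for animation montages, stamina, weapon handling and facing.
; High-priority montages play unless that same montage is already playing and are recorded, while regular montages play only when no montage is active.
; Stamina replenishes in capped steps, and dropping a weapon detaches it and clears its reference.
; Desired rotation follows last movement input or current facing, though HasMovementInput's check is unwired and StartRotatingWithLimit is empty.
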(fn ConstructionScript)

(fn PlayHighPriorityMontage
  (params (Montage :type Anim%20Montage%20Object%20Reference) (StartSectionName :type Name) (InPlayRate :type Float%20%28single-precision%29))
  (if (not (Animation|Montage|MontageIsPlaying (Components|SkeletalMesh|GetAnimInstance (Variables|Character|GetMesh)) Montage))
    (bind _output_get (Variables|Default|SetHighPriorityMontage Montage))
    (bind _returnvalue (Animation|PlayAnimMontage _output_get InPlayRate StartSectionName))
    (return _returnvalue)))

(fn TryPlayAnimMontage
  (params (Montage :type Anim%20Montage%20Object%20Reference) (StartSectionName :type Name) (InPlayRate :type Float%20%28single-precision%29))
  (if (not (Animation|Montage|MontageIsPlaying (Components|SkeletalMesh|GetAnimInstance (Variables|Character|GetMesh)) 0))
    (bind _returnvalue (Animation|PlayAnimMontage Montage InPlayRate StartSectionName))
    (return _returnvalue)))

(fn Replenish
  (if (>= (Variables|Default|GetStamina) 1e+02)
    (Variables|Default|SetStamina 1e+02)
    (else
      (Variables|Default|SetStamina (+ (Variables|Default|GetStamina) 1.0)))))

(fn DropCurrentWeapon
  (Transformation|DetachFromActor (Variables|Default|GetWeapon) "KeepRelative" "KeepRelative" "KeepRelative")
  (Variables|Default|SetWeapon 0))

(fn GetDesiredRotation
  (if (Utilities|HasMovementInput)
    (return (Math|Conversions|RotationFromXVector (Class|Pawn|GetLastMovementInputVector)))
    (else
      (return (Transformation|GetActorRotation)))))

(fn StartRotatingwithLimit
  (params (MaxPossibleRotation :type Float%20%28single-precision%29) (MaxDegreesPerSecond :type Float%20%28single-precision%29))
  (return))