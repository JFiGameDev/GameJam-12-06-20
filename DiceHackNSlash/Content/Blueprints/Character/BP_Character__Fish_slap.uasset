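; Character Blueprint that performs a melee slap attack on left mouse click by playing a sword slash montage on the mesh.
; The montage's notify begin fires a sphere trace on the Camera channel from the WeaponSlot socket, with persistent debug drawing.
; The trace end multiplies the sum of socket location and forward vector, rather than offsetting along forward.
; The hit actor receives damage and a damage event is reported to AI perception.
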(event EventBeginPlay
  (|CallParentFunction) ; This node is disabled and will not be called.\nDrag off pins to build functionality.
)

(event Collision|EventActorBeginOverlap
  (params (OtherActor :type Actor%20Object%20Reference)))

(event EventTick
  (params (DeltaSeconds :type Float%20%28single-precision%29))
  (|CallParentFunction DeltaSeconds) ; This node is disabled and will not be called.\nDrag off pins to build functionality.
)

(event Input|MouseEvents|LeftMouseButton
  (params (Key :type Key%20Structure :default "None"))
  (bind _mesh (Variables|Character|GetMesh))
  (bind _returnvalue (Transformation|GetSocketLocation _mesh "WeaponSlot"))
  (:Pressed
    (Animation|Montage|PlayMontage (Variables|Character|GetMesh) "/Game/Character/Animations/Stable_Sword_Outward_Slash_Anim_Montage.Stable_Sword_Outward_Slash_Anim_Montage"
      (:OnNotifyBegin
        (bind _outhit (Collision|SphereTraceByChannel _returnvalue (* (+ _returnvalue (Math|Vector|GetForwardVector (Transformation|GetActorRotation))) 5e+01) 4e+01 "TraceTypeQuery2" false 0 "Persistent"))
        (Game|Damage|ApplyDamage (.hitactor _outhit) 0.5 0 0)
        (Class|AISenseDamage|ReportDamageEvent (.hitactor _outhit) self 0.0 (.tracestart _outhit))))))

(fn ConstructionScript
  (|CallParentFunction))