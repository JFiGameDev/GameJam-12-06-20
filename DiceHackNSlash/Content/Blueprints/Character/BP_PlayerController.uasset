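; Player controller that relays player input to the possessed BP_Character.
; On possession it casts the pawn to BP_Character and caches the reference.
; Movement axes, attack press and release, and roll on button release forward straight to character functions.
; Both mouse axis events share a single MouseRotate call, leaving the gameplay logic to the character.
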(event EventPossess
  (params (PossessedPawn :type Pawn%20Object%20Reference))
  ;[1 1 1] Get Character Ref
  (Variables|Default|SetCharacterRef (.AsBP%20Character (Utilities|Casting|CastToBP_Character PossessedPawn))))

(event Input|ActionEvents|InputActionAttackInput
  (params (Key :type Key%20Structure :default "None"))
  (bind _characterref (Variables|Default|GetCharacterRef))
  ;[1 1 1] Input
  (:Pressed
    (Default|Attack _characterref))
  (:Released
    (Default|AttackReleased _characterref)))

(event Input|ActionEvents|InputActionRollInput
  (params (Key :type Key%20Structure :default "None"))
  ;[1 1 1] Input
  (:Released
    (Default|Roll (Variables|Default|GetCharacterRef))))

(event Input|AxisEvents|InputAxisMoveForward
  (params (AxisValue :type Float%20%28single-precision%29))
  ;[1 1 1] Input
  (Default|MoveUp/Down (Variables|Default|GetCharacterRef) AxisValue))

(event Input|AxisEvents|InputAxisMoveRight
  (params (AxisValue :type Float%20%28single-precision%29))
  ;[1 1 1] Input
  (Default|MoveLeft/Right (Variables|Default|GetCharacterRef) AxisValue))

(event Input|MouseEvents|MouseX
  (params (AxisValue :type Float%20%28single-precision%29))
  ;[1 1 1] Input
  (Default|MouseRotate (Variables|Default|GetCharacterRef) AxisValue (stale Input|MouseEvents|MouseY AxisValue)))

(event Input|MouseEvents|MouseY
  (params (AxisValue :type Float%20%28single-precision%29))
  ;[1 1 1] Input
  (Default|MouseRotate (Variables|Default|GetCharacterRef) (stale Input|MouseEvents|MouseX AxisValue) AxisValue))

(fn ConstructionScript)