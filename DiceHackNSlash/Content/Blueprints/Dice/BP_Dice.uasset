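; Physics-simulated die actor that reports which face it landed on.
; When the mesh sleeps, it takes the socket with the highest world Z as the showing face and broadcasts it through DiceHasLanded.
; It then spawns an explosion effect and stops simulating physics.
; While simulating, hits on components not tagged BestSurface push the die along the impact normal, bouncing it off those surfaces.
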(event OnComponentHit(Die)
  (params (HitComponent :type Primitive%20Component%20Object%20Reference) (OtherActor :type Actor%20Object%20Reference) (OtherComp :type Primitive%20Component%20Object%20Reference) (NormalImpulse :type Vector :default "0, 0, 0") (Hit :type Hit%20Result%20Structure%20%28by%20ref%29))
  (bind _die (Variables|Default|GetDie))
  (if (not (Components|ComponentHasTag OtherComp "BestSurface"))
    (if (Physics|IsSimulatingPhysics _die "None")
      (Physics|AddImpulse _die (* (.ImpactNormal (Collision|BreakHitResult Hit)) 1e+04) "None" false))))

(event OnComponentSleep(Die)
  (params (SleepingComponent :type Primitive%20Component%20Object%20Reference) (BoneName :type Name :default "None"))
  (bind _die (Variables|Default|GetDie))
  (bind _returnvalue (Transformation|GetWorldTransform _die))
  (Variables|Default|SetHighest -9999.0)
  (for _array_element (Transformation|GetAllSocketNames _die)
    (if (> (.z (Transformation|GetSocketLocation _die _array_element)) (Variables|Default|GetHighest))
      (Variables|Default|SetHighest (.z (Transformation|GetSocketLocation _die _array_element)))
      (Variables|Default|SetFaceShowing _array_element)))
  (Default|CallDiceHasLanded (Variables|Default|GetFaceShowing) self)
  (Effects|SpawnEmitteratLocation "/Game/StarterContent/Particles/P_Explosion.P_Explosion" (.location _returnvalue) (.rotation _returnvalue))
  (Physics|SetSimulatePhysics _die false))

(event EventBeginPlay)

(event Collision|EventActorBeginOverlap
  (params (OtherActor :type Actor%20Object%20Reference)))

(event EventTick
  (params (DeltaSeconds :type Float%20%28single-precision%29)))

(fn ConstructionScript)