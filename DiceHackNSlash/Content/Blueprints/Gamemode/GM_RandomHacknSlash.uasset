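; Game mode for a dice-driven hack-and-slash that randomizes the player's loadout and handles spawning between levels.
; Two events use a dice roll to pick the equipped weapon from a list or multiply the character's current health.
; Both get the player through a helper that returns only the first controller despite looping.
; The ChoosePlayerStart override matches start tags to the game instance's DoorID, falling back to the first start found.
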(event Custom|AssignRandomWeapon
  (bind _playercontroller (CallFunction|FGetPlayerControllers))
  (bind _rolloutcome (CallFunction|FDiceRollFunction))
  (Variables|/Game/Blueprints/Character/Inventory.Inventory_C|SetEquippedWeapon (Variables|/Game/Blueprints/Character/BP_PlayerController.BP_PlayerController_C|GetInventory _playercontroller) (Utilities|Array|Get(acopy) (Variables|Default|GetWeaponList) _rolloutcome)))

(event Custom|AssignRandomHealth
  (bind _playercontroller (CallFunction|FGetPlayerControllers))
  (bind _asbp_character (Utilities|Casting|CastToBP_Character (Pawn|GetControlledPawn _playercontroller)))
  (Utilities|IsValid _asbp_character
    (:Is%20Valid
      (bind _rolloutcome (CallFunction|FDiceRollFunction))
      (Variables|/Game/Blueprints/Character/BP_Character.BP_Character_C|SetHealth _asbp_character (* _rolloutcome (Variables|/Game/Blueprints/Character/BP_Character.BP_Character_C|GetHealth _asbp_character))))))

(fn ConstructionScript)

(fn FGetPlayerControllers
  (bind _returnvalue (Class|GameModeBase|GetNumPlayers))
  (for _index (range 0 _returnvalue)
    (bind _asbp_player_controller (Utilities|Casting|CastToBP_PlayerController (Game|GetPlayerController _index)))
    (return _asbp_player_controller)))

(fn ChoosePlayerStart
  (params (Player :type Controller%20Object%20Reference))
  ;[1 1 1] Player start when going into another level
  (bind _asdicemaname_instance (Utilities|Casting|CastToDicemanameInstance (Game|GetGameInstance)))
  (bind _outactors (Actor|GetAllActorsOfClass "/Script/Engine.PlayerStart"))
  (for _array_element _outactors
    (if (Utilities|Name|Equal(Name) (Variables|/Script/Engine.PlayerStart|GetPlayerStartTag _array_element) (Variables|/Game/Blueprints/Portals/DicemanameInstance.DicemanameInstance_C|GetDoorID _asdicemaname_instance))
      (return _array_element)))
  (return (Utilities|Array|Get(acopy) _outactors)))