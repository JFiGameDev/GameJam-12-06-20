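; BP_FallingPlatform is a trap Blueprint, named as a falling platform, that starts a timeline when the player enters its trigger.
; BeginPlay caches the player's BP_Character and the Trap's world location.
; On Trigger overlap it waits a configurable delay, then plays TrapTimeLine if the overlapping actor is that player.
; The timeline has no update logic here, and the stored location is never read.
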(event OnComponentBeginOverlap(Trigger)
  (params (OverlappedComponent :type Primitive%20Component%20Object%20Reference) (OtherActor :type Actor%20Object%20Reference) (OtherComp :type Primitive%20Component%20Object%20Reference) (OtherBodyIndex :type Integer) (bFromSweep :type Boolean) (SweepResult :type Hit%20Result%20Structure%20%28by%20ref%29))
  (Utilities|FlowControl|Delay (Variables|TrapSettings|GetDelay))
  (if (== OtherActor (Variables|Reference|GetPlayerRef))
    (Timeline|TrapTimeLine Play)))

(event EventBeginPlay
  (bind _asbp_character (Utilities|Casting|CastToBP_Character (Game|Player|GetPlayerPawn 0)))
  (Variables|Reference|SetPlayerRef _asbp_character)
  (Variables|Target|SetTrap%20Loacation (Transformation|GetWorldLocation (Variables|/Script/Engine.Actor|GetRootComponent (Variables|Target|GetTrap)))))

(fn ConstructionScript)